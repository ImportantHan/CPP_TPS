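; BP_AI is an AI pawn that wanders the navmesh and heads toward the player when it perceives one.
; On BeginPlay it picks a random reachable point nearby and starts AIMoveTo, repeating with a new point whenever a move succeeds or fails.
; An AI Perception update for BP_TPSPlayer replaces the target with that player's current location and restarts the move, without checking whether the stimulus was gained or lost.
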(event OnTargetPerceptionUpdated(AIPerception)
  (params (Actor :type Actor%20Object%20Reference) (Stimulus :type AI%20Stimulus%20Structure))
  (bind _asbp_tpsplayer (Utilities|Casting|CastToBP_TPSPlayer Actor))
  (Variables|Default|SetTarget (Transformation|GetActorLocation _asbp_tpsplayer))
  (CallFunction|AIMove))

(event Custom|AIMove
  (AI|AIMoveTo self (Variables|Default|GetTarget) 0 5.0 false
    (:OnSuccess
      _)
    (:OnFail
      _))
  (CallFunction|UpdateRandomLocation)
  (CallFunction|AIMove))

(event EventBeginPlay
  (CallFunction|UpdateRandomLocation)
  (CallFunction|AIMove))

(event Collision|EventActorBeginOverlap
  (params (OtherActor :type Actor%20Object%20Reference)))

(event EventTick
  (params (DeltaSeconds :type Float%20%28single-precision%29)))

(fn ConstructionScript)

(fn UpdateRandomLocation
  (Variables|Default|SetTarget (.RandomLocation (AI|Navigation|GetRandomReachablePointinRadius (Transformation|GetActorLocation) 5e+02 0 0))))